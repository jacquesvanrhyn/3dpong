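; Top_Paddle is an AI-controlled paddle that follows balls along the X axis.
; Each Tick, if it strays past its fixed X limits on either side, it is set back just inside.
; Otherwise it finds all Ball actors and, for each, adds an X impulse to its StaticMesh from the clamped offset to that ball, scaled by AIPaddleSpeed.
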(event `self.ReceiveActorBeginOverlap`
  (params (OtherActor :type "Actor Object Reference")))

(event `self.ReceiveBeginPlay`)

(event `self.ReceiveTick`
  (params (DeltaSeconds :type "Float (single-precision)"))
  (if (> (.x (`self.K2_GetActorLocation`)) 400.0)
    (`self.K2_SetActorLocation` (`KismetMathLibrary.MakeVector` 399.0 (.y (`self.K2_GetActorLocation`)) (.z (`self.K2_GetActorLocation`))))
    (elif (< (.x (`self.K2_GetActorLocation`)) -400.0)
      (`self.K2_SetActorLocation` (`KismetMathLibrary.MakeVector` -399.0 (.y (`self.K2_GetActorLocation`)) (.z (`self.K2_GetActorLocation`))))
      (else
        (bind _outactors (`GameplayStatics.GetAllActorsOfClass` "/Game/Blueprints/Ball.Ball_C"))
        (for _array_element _outactors
          (`PrimitiveComponent.AddImpulse` (`self.StaticMesh`) (* (`KismetMathLibrary.MakeVector` (`KismetMathLibrary.FClamp` (- (.x (`self.K2_GetActorLocation` _array_element)) (.x (`self.K2_GetActorLocation`))) -3.0 3.0)) (`self.AI_Paddle_Speed`)) "None" false))))))

(fn `UserConstructionScript`)