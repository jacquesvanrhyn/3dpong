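; Ball actor for a sudden-death Pong game that also keeps score and ends the match.
; Overlaps flip its physics velocity off boundaries, goals and paddles; paddle hits add paddle X velocity plus random spread, and top-paddle hits speed up Y.
; Goal overlaps update tagged TextRenderActor scoreboards, and a side passing two points sets Gameover.
; Tick then stops the ball and reloads the Main level after a delay.
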(event `self.ReceiveTick`
  (params (DeltaSeconds :type "Float (single-precision)"))
  (if (`self.Gameover`)
    (`PrimitiveComponent.SetPhysicsLinearVelocity` (`self.StaticMesh`) (0.0 0.0 0.0) false "None")
    (`KismetSystemLibrary.Delay` 2.0)
    (`GameplayStatics.OpenLevel` "Main")))

(event `self.ReceiveBeginPlay`
  (`PrimitiveComponent.SetPhysicsLinearVelocity` (`self.StaticMesh`) (`KismetMathLibrary.MakeVector` 0.0 (`self.ball_speed`)) false "None")
  (`KismetSystemLibrary.PrintString` "Good luck!" true true (struct :`G` 0.66 :`B` 1.0 :`A` 1.0) 4.0)
  (`KismetSystemLibrary.PrintString` "Use the right and left arrows to move your paddle." true true (struct :`G` 0.66 :`B` 1.0 :`A` 1.0) 4.0)
  (`KismetSystemLibrary.PrintString` "Welcome to sudden death pong where every time the enemy hits the ball, the ball moves faster!" true true (struct :`G` 0.66 :`B` 1.0 :`A` 1.0) 4.0))

(event `self.ReceiveActorBeginOverlap`
  (params (OtherActor :type "Actor Object Reference"))
  (bind _asbottom_paddle (cast `/Game/Blueprints/Bottom_Paddle` OtherActor)
    (:`then`
      (bind _returnvalue (`PrimitiveComponent.GetPhysicsLinearVelocity` (`/Game/Blueprints/Bottom_Paddle.Paddle_mesh` _asbottom_paddle) "None"))
      (bind _returnvalue_2 (`PrimitiveComponent.GetPhysicsLinearVelocity` (`self.StaticMesh`) "None"))
      (`PrimitiveComponent.SetPhysicsLinearVelocity` (`self.StaticMesh`) (`KismetMathLibrary.MakeVector` (+ (`KismetMathLibrary.RandomFloatInRange` -100.0 100.0) (.x _returnvalue)) (* (.y _returnvalue_2) -1.0) (.z _returnvalue_2)) false "None"))
    (:`CastFailed`
      (cast `/Game/Blueprints/Boundary_mesh` OtherActor
        (:`then`
          (bind _returnvalue_3 (`PrimitiveComponent.GetPhysicsLinearVelocity` (`self.StaticMesh`) "None"))
          (`PrimitiveComponent.SetPhysicsLinearVelocity` (`self.StaticMesh`) (`KismetMathLibrary.MakeVector` (* (.x _returnvalue_3) -1.0) (.y _returnvalue_3) (.z _returnvalue_3)) false "None"))
        (:`CastFailed`
          (cast `/Game/Blueprints/Top_goal` OtherActor
            (:`then`
              (bind _returnvalue_4 (`PrimitiveComponent.GetPhysicsLinearVelocity` (`self.StaticMesh`) "None"))
              (`PrimitiveComponent.SetPhysicsLinearVelocity` (`self.StaticMesh`) (`KismetMathLibrary.MakeVector` (.x _returnvalue_4) (* (.y _returnvalue_4) -1.0) (.z _returnvalue_4)) false "None")
              (set `self.Bottom_Score` (+ (`self.Bottom_Score`) 1))
              (bind _outactors (`GameplayStatics.GetAllActorsOfClass` "/Script/Engine.TextRenderActor"))
              (for _array_element _outactors
                (if (`ActorComponent.ComponentHasTag` (`TextRenderActor.TextRender` _array_element) "bottom_score")
                  (`TextRenderComponent.K2_SetText` (`TextRenderActor.TextRender` _array_element) (`KismetTextLibrary.Conv_IntToText` (`self.Bottom_Score`)))
                  (if (> (`self.Bottom_Score`) 2)
                    (`KismetSystemLibrary.PrintString` "Human Wiins!")
                    (set `self.Gameover` true)))))
            (:`CastFailed`
              (cast `/Game/Blueprints/Bottom_goal` OtherActor
                (:`then`
                  (bind _returnvalue_5 (`PrimitiveComponent.GetPhysicsLinearVelocity` (`self.StaticMesh`) "None"))
                  (`PrimitiveComponent.SetPhysicsLinearVelocity` (`self.StaticMesh`) (`KismetMathLibrary.MakeVector` (.x _returnvalue_5) (* (.y _returnvalue_5) -1.0) (.z _returnvalue_5)) false "None")
                  (set `self.Top_Score` (+ (`self.Top_Score`) 1))
                  (bind _outactors_2 (`GameplayStatics.GetAllActorsOfClass` "/Script/Engine.TextRenderActor"))
                  (for _array_element_2 _outactors_2
                    (if (`ActorComponent.ComponentHasTag` (`TextRenderActor.TextRender` _array_element_2) "top_score")
                      (`TextRenderComponent.K2_SetText` (`TextRenderActor.TextRender` _array_element_2) (`KismetTextLibrary.Conv_IntToText` (`self.Top_Score`)))
                      (if (> (`self.Top_Score`) 2)
                        (`KismetSystemLibrary.PrintString` "Deep Blue Wins!")
                        (set `self.Gameover` true)))))
                (:`CastFailed`
                  (bind _astop_paddle (cast `/Game/Blueprints/Top_Paddle` OtherActor))
                  (bind _returnvalue_6 (`PrimitiveComponent.GetPhysicsLinearVelocity` (`/Game/Blueprints/Top_Paddle.StaticMesh` _astop_paddle) "None"))
                  (bind _returnvalue_7 (`PrimitiveComponent.GetPhysicsLinearVelocity` (`self.StaticMesh`) "None"))
                  (`PrimitiveComponent.SetPhysicsLinearVelocity` (`self.StaticMesh`) (`KismetMathLibrary.MakeVector` (+ (`KismetMathLibrary.RandomFloatInRange` -100.0 100.0) (.x _returnvalue_6)) (* (.y _returnvalue_7) -1.1) (.z _returnvalue_7)) false "None"))))))))))

(fn `UserConstructionScript`)